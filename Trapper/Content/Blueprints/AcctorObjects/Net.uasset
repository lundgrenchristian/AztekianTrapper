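; Net actor that expands after spawning and catches players other than its instigator.
; A timeline started on BeginPlay widens the mesh in Y and Z while keeping it thin in X.
; On overlap, the server checks the player's CurrentState and calls either CaughtInNet or AlienCaughtInNet.
; A hit on the net mesh destroys the actor after a short delay.
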(event OnComponentHit(NetMesh)
  (params (HitComponent :type Primitive%20Component%20Object%20Reference) (OtherActor :type Actor%20Object%20Reference) (OtherComp :type Primitive%20Component%20Object%20Reference) (NormalImpulse :type Vector :default "0, 0, 0") (Hit :type Hit%20Result%20Structure%20%28by%20ref%29))
  (Utilities|FlowControl|Delay 0.2)
  (Actor|DestroyActor))

(event EventBeginPlay
  (bind _expand (Timeline|ExpandNetOverTime PlayFromStart)
    (:Update
      (CallFunction|NetExpand _expand))))

(event Collision|EventActorBeginOverlap
  (params (OtherActor :type Actor%20Object%20Reference))
  (Networking|SwitchHasAuthority
    (:Authority
      (bind _asplayer (Utilities|Casting|CastToPlayer OtherActor))
      (Utilities|IsValid _asplayer
        (:Is%20Valid
          (if (!= OtherActor (Variables|Actor|GetInstigator))
            (bind _asplayer_2 (Utilities|Casting|CastToPlayer OtherActor))
            (if (Utilities|Enum|Equal(Enum) (Variables|/Game/BluePrints/Player.Player_C|GetCurrentState _asplayer_2) "NewEnumerator0")
              (Default|CaughtinNet _asplayer)
              (elif (Utilities|Enum|Equal(Enum) (Variables|/Game/BluePrints/Player.Player_C|GetCurrentState _asplayer_2) "NewEnumerator3")
                (Default|AlienCaughtinNet _asplayer_2)))))))))

(event EventTick
  (params (DeltaSeconds :type Float%20%28single-precision%29)))

(fn ConstructionScript)

(fn NetExpand
  (params (Float :type Float%20%28single-precision%29))
  (Transformation|SetWorldScale3D (Variables|Default|GetNetMesh) (Math|Vector|MakeVector 0.02 Float Float)))