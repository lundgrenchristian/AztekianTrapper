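; GM is the game mode for a timed multiplayer match in which the current artifact holder earns points.
; It spawns and possesses a pawn per login at an indexed player start, then a one-time countdown unfreezes everyone and shows timer and ability UI.
; A looping one-second timer decrements the GameState clock, scores the holder once SwitchTag has assigned one, and freezes all players at zero.
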(event Custom|Countdown
  ;[1 1 1] Countdown
  (if (not (Variables|Default|GetStarted))
    (for _array_element (Variables|Default|GetPlayers)
      (Default|ShowCountdown _array_element))
    (Variables|Default|SetStarted true)
    (Utilities|FlowControl|Delay 3.0)
    (CallFunction|UnFreeze)))

(event Custom|UnFreeze
  ;[1 1 1] UnFreeze controls
  (for _array_element (Variables|Default|GetPlayers)
    (Default|UnFreeze _array_element))
  ;[1 1 1] Match timer
  (Variables|/Game/BluePrints/GS_Base.GS_Base_C|SetCurrentTime (Variables|Default|GetGS_Base) (Variables|Default|GetMatchTimer))
  (bind _returnvalue (Utilities|Time|SetTimerbyEvent (delegate Custom|Count) 1.0 true))
  (CallFunction|ShowTimers))

(event Custom|Count
  ;[1 1 1] Match timer
  (bind _result (Math|Integer|DecrementInt (Variables|/Game/BluePrints/GS_Base.GS_Base_C|GetCurrentTime (Variables|Default|GetGS_Base)))
    (:%20%20
      (Utilities|FlowControl|Sequence
        (:then_0
          (if (Variables|Default|GetPointStart)
            (Math|Integer|IncrementInt (Variables|/Game/BluePrints/PC.PC_C|GetPoints (Variables|/Game/BluePrints/GS_Base.GS_Base_C|GetArtifactHolder (Variables|Default|GetGS_Base)))
              (:%20%20
                (if (== _result 0) :!label _label
                  (Utilities|Time|PauseTimerbyHandle (stale Custom|UnFreeze _returnvalue))
                  (CallFunction|Freeze))))))
        (:then_1
          (if (not (Variables|Default|GetPointStart))
            (goto _label)))))))

(event Custom|ShowTimers
  ;[0.9333 0.957 1] Show match timer and abilities
  (for _array_element (Variables|Default|GetPlayers)
    (Default|ShowInfo _array_element)
    (Default|ShowNet _array_element)
    (Default|ShowDash _array_element)
    (Default|ShowBlink _array_element)
    (Default|ShowCopy _array_element)))

(event Custom|Freeze
  ;[1 1 1] Freeze input after timer ends
  (for _array_element (Variables|Default|GetPlayers)
    (Default|Freeze _array_element)))

(event Custom|SwitchTag
  (params (ArtifactHolder :type PC%20Object%20Reference))
  ;[1 1 1] Swap Alien Tag
  (Variables|Default|SetPointStart true)
  (Variables|/Game/BluePrints/GS_Base.GS_Base_C|SetArtifactHolder (Variables|Default|GetGS_Base) ArtifactHolder))

(event EventPostLogin
  (params (NewPlayer :type Player%20Controller%20Object%20Reference))
  ;[1 1 1] Spawn player and assign position
  (bind _aspc (Utilities|Casting|CastToPC NewPlayer))
  (Utilities|Array|Add (Variables|Default|GetPlayers) _aspc)
  (bind _returnvalue (Game|SpawnActorfromClass "/Game/BluePrints/Player.Player_C" (Transformation|GetActorTransform (Class|GameModeBase|FindPlayerStart NewPlayer (Utilities|String|ToString(Integer) (- (Utilities|Array|Length (Variables|Default|GetPlayers)) 1)))) "Undefined" 0 0))
  (Pawn|Possess NewPlayer _returnvalue))

(event EventBeginPlay
  ;[1 1 1] Assign GameState
  (bind _asgs_base (Utilities|Casting|CastToGS_Base (Game|GetGameState)))
  (Variables|Default|SetGS_Base _asgs_base))

(fn ConstructionScript)