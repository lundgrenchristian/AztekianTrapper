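; Player controller for a session-based match game with artifact holder and alien capture, handling HUD widgets, pawn input freezing and leaving to the main menu.
; Enter starts the GameMode countdown, U opens settings, and E calls CaptureAlien on the Player unless this controller holds the artifact.
; Tick drives net, dash, blink and copy cooldowns through 0.1-second Delays, adding a new widget on each update without removing the previous one.
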(event Custom|ShowCountdown
  ;[1 1 1] Show countdown on start
  (bind _returnvalue (UserInterface|CreateWidget "/Game/Blueprints/Widgets/W_showcountdown.W_showcountdown_C"))
  (UserInterface|Viewport|AddtoViewport _returnvalue 0))

(event Custom|UnFreeze
  ;[1 1 1] Unfreeze the movement
  (Input|EnableInput (Pawn|GetControlledPawn) self))

(event Custom|Update%20CopyWidget
  ;[0 1 1] Show cooldown on copy
  (if (Variables|Default|GetCopyUsed)
    (Utilities|FlowControl|Delay 0.1)
    (Variables|Default|SetCopyCooldown (- (Variables|Default|GetCopyCooldown) 0.1))
    (CallFunction|ShowCopy)))

(event Custom|ShowCopy
  ;[0 1 1] Show copy widget
  (bind _returnvalue (UserInterface|CreateWidget "/Game/Blueprints/Widgets/W_Copy.W_Copy_C"))
  (UserInterface|Viewport|AddtoViewport _returnvalue 0))

(event Custom|Show%20Crosshair
  ;[1 1 1] Crosshair
  (bind _returnvalue (UserInterface|CreateWidget "/Game/Blueprints/Widgets/W_Crosshair.W_Crosshair_C"))
  (UserInterface|Viewport|AddtoViewport _returnvalue 0))

(event Custom|ShowWinnerWidget
  (params (Won :type Boolean))
  ;[1 1 1] Show winner widget
  (Viewport|RemoveAllWidgets)
  (bind _returnvalue (UserInterface|CreateWidget "/Game/Blueprints/Widgets/W_winner.W_winner_C" 0 Won))
  (UserInterface|Viewport|AddtoViewport _returnvalue 0))

(event Custom|BackToMainMenu
  ;[1 1 1] Destroy session and return to main menu
  (|DestroySession self
    (:OnSuccess
      (Development|PrintString "successfully left session")
      (Game|OpenLevel(byName) "MainMenu"))
    (:OnFailure
      (Development|PrintString "Failed to leave session"))))

(event Custom|ShowInfo
  ;[1 1 1] Show points and timer
  (bind _returnvalue (UserInterface|CreateWidget "/Game/Blueprints/Widgets/W_info.W_info_C"))
  (UserInterface|Viewport|AddtoViewport _returnvalue 0))

(event Custom|Freeze
  ;[1 1 1] Freeze input
  (Input|DisableInput (Pawn|GetControlledPawn) self))

(event Custom|Show%20Net
  ;[0 1 1] Show net widget
  (bind _returnvalue (UserInterface|CreateWidget "/Game/Blueprints/Widgets/W_NetShoot.W_NetShoot_C"))
  (UserInterface|Viewport|AddtoViewport _returnvalue 0))

(event Custom|Update%20NetWidget
  ;[0 1 1] Show cooldown on net
  (if (Variables|Default|GetNetUsed)
    (Utilities|FlowControl|Delay 0.1)
    (Variables|Default|SetNetCooldown (- (Variables|Default|GetNetCooldown) 0.1))
    (CallFunction|ShowNet)))

(event Custom|Update%20DashWidget
  ;[0 1 1] Show cooldown on dash
  (if (Variables|Default|GetDashUsed)
    (Utilities|FlowControl|Delay 0.1)
    (Variables|Default|SetDashCooldown (- (Variables|Default|GetDashCooldown) 0.1))
    (CallFunction|ShowDash)))

(event Custom|Show%20Dash
  ;[0 1 1] Show dash widget
  (bind _returnvalue (UserInterface|CreateWidget "/Game/Blueprints/Widgets/W_Dash.W_Dash_C"))
  (UserInterface|Viewport|AddtoViewport _returnvalue 0))

(event Custom|ShowBlink
  ;[0 1 1] Show blink widget
  (bind _returnvalue (UserInterface|CreateWidget "/Game/Blueprints/Widgets/W_Blink.W_Blink_C"))
  (UserInterface|Viewport|AddtoViewport _returnvalue 0))

(event Custom|Update%20BlinkWidget
  ;[0 1 1] Show cooldown on blink
  (if (Variables|Default|GetBlinkUsed)
    (Utilities|FlowControl|Delay 0.1)
    (Variables|Default|SetBlinkCooldown (- (Variables|Default|GetBlinkCooldown) 0.1))
    (CallFunction|ShowBlink)))

(event EventBeginPlay
  ;[1 1 1] Set GameState
  (Input|SetInputModeGameOnly self)
  (bind _asgs_base (Utilities|Casting|CastToGS_Base (Game|GetGameState)))
  (Variables|Default|SetGS_Base _asgs_base))

(event EventTick
  (params (DeltaSeconds :type Float%20%28single-precision%29))
  ;[1 1 1] On Tick update
  (CallFunction|UpdateDashWidget)
  (CallFunction|UpdateNetWidget)
  (CallFunction|UpdateBlinkWidget)
  (CallFunction|UpdateCopyWidget))

(event Input|KeyboardEvents|Enter
  (params (Key :type Key%20Structure :default "None"))
  ;[1 1 1] Start game
  (:Pressed
    (bind _asgm (Utilities|Casting|CastToGM (Game|GetGameMode)))
    (Default|Countdown _asgm)))

(event Input|KeyboardEvents|E
  (params (Key :type Key%20Structure :default "None"))
  ;[1 1 1] E to interact
  (:Pressed
    (if (not (== (Variables|/Game/Blueprints/GS_Base.GS_Base_C|GetArtifactHolder (Variables|Default|GetGS_Base)) self))
      (bind _asplayer (Utilities|Casting|CastToPlayer (Pawn|GetControlledPawn)))
      (Default|CaptureAlien _asplayer))))

(event Input|KeyboardEvents|U
  (params (Key :type Key%20Structure :default "None"))
  (:Pressed
    (bind _returnvalue (UserInterface|CreateWidget "/Game/Blueprints/Widgets/W_SettingsMenu.W_SettingsMenu_C"))
    (UserInterface|Viewport|AddtoViewport _returnvalue 0)
    (Variables|Default|SetbShowMouseCursor true)))

(fn ConstructionScript)