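; LifeformUnknown is a character that launches itself in arcing jumps.
; On BeginPlay in the Plan to Jump state, it traces downward at a random, range-clamped spot and leaps to the hit using SuggestProjectileVelocityCustomArc.
; Event 111 launches it horizontally toward its FollowCamera's position with added height, gated by a DoOnce that resets on landing.
; That event's only call and another launch test are disconnected.
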(event Custom|Jumpnoww
  (params (Velocity :type Vector))
  (Character|LaunchCharacter Velocity false false))

(event Custom|111
  (bind _returnvalue (Transformation|GetActorLocation))
  (Utilities|FlowControl|DoOnce false
    (:Completed
      (bind _outlaunchvelocity (Game|SuggestProjectileVelocityCustomArc _returnvalue (+ _returnvalue (+ (* (Math|Vector|Normalize (* (- (Transformation|GetWorldLocation (Variables|Default|GetFollowCamera)) (Transformation|GetActorLocation)) "1.000000,1.000000,0.000000")) "1000.000000,1000.000000,1.000000") "0, 0,500.000000")) 0.0 0.5))
      (Character|LaunchCharacter _outlaunchvelocity true true))))

(event EventOnLanded
  (params (Hit :type Hit%20Result%20Structure%20%28by%20ref%29))
  (bind _returnvalue (Transformation|GetActorLocation))
  (Utilities|FlowControl|DoOnce false) ; enters at Reset
)

(event EventBeginPlay
  (bind _returnvalue (Math|Random|RandomFloatinRange 5e+03 1e+04))
  (bind _returnvalue_2 (Math|Random|RandomUnitVector))
  (bind _capsulecomponent (Variables|Default|GetCapsuleComponent))
  (bind _returnvalue_3 (* _returnvalue_2 _returnvalue))
  (bind _returnvalue_4 (Transformation|GetWorldLocation _capsulecomponent))
  (bind _returnvalue_5 (+ _returnvalue_3 _returnvalue_4))
  (bind _returnvalue_6 (Math|Float|Clamp(Float) (.y _returnvalue_5) -1e+04 1e+04))
  (bind _returnvalue_7 (Math|Float|Clamp(Float) (.x _returnvalue_5) -1e+04 1e+04))
  (switch Utilities|FlowControl|Switch|SwitchonLifeformStates (Variables|Default|GetCurrent%20State)
    (:NewEnumerator0
      (bind (_outhit _returnvalue_8) (Collision|LineTraceByChannel (Math|Vector|MakeVector _returnvalue_7 _returnvalue_6 1e+04) (Math|Vector|MakeVector _returnvalue_7 _returnvalue_6 0.0) "TraceTypeQuery1" false 0 "Persistent"))
      (if _returnvalue_8
        (bind _outlaunchvelocity (Game|SuggestProjectileVelocityCustomArc (Transformation|GetWorldLocation (Variables|Default|GetCapsuleComponent)) (.Location (Collision|BreakHitResult _outhit)) 0.0 0.5))
        (CallFunction|Jumpnoww _outlaunchvelocity)))))

(fn ConstructionScript
  (|CallParentFunction))