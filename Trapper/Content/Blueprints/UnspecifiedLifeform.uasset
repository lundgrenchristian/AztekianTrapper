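; UnspecifiedLifeform is a character that roams by making long, repeated ballistic leaps to random ground points.
; In its Plan to Jump state, on BeginPlay and each landing, it traces downward at random positions clamped to a fixed area, retrying if too close.
; A trace hit feeds SuggestProjectileVelocityCustomArc, whose velocity launches the character through JumpEvent.
; Tick turns the actor to face its velocity, and Jumpnoww is an empty stub.
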(event Custom|JumpEvent
  (params (Velocity :type Vector))
  (Character|LaunchCharacter Velocity true true))

(event EventTick
  (params (DeltaSeconds :type Float%20%28single-precision%29))
  (bind _returnvalue (Transformation|GetActorLocation))
  (Transformation|SetActorRotation (Math|Rotator|FindLookatRotation _returnvalue (+ _returnvalue (Transformation|GetVelocity)))))

(event EventBeginPlay
  (bind _returnvalue (Math|Random|RandomFloatinRange 5e+03 7.5e+03))
  (bind _returnvalue_2 (Math|Random|RandomUnitVector))
  (bind _capsulecomponent (Variables|Collision|GetCapsuleComponent))
  (bind _returnvalue_3 (* _returnvalue_2 _returnvalue))
  (bind _returnvalue_4 (Transformation|GetWorldLocation _capsulecomponent))
  (bind _returnvalue_5 (+ _returnvalue_3 _returnvalue_4))
  (bind _returnvalue_6 (Math|Float|Clamp(Float) (.y _returnvalue_5) -5e+03 5e+03))
  (bind _returnvalue_7 (Math|Float|Clamp(Float) (.x _returnvalue_5) -5e+03 5e+03))
  (switch Utilities|FlowControl|Switch|SwitchonLifeformStates (Variables|Default|GetCurrent%20State) :!label _label
    (:NewEnumerator0
      (bind (_outhit _returnvalue_8) (Collision|LineTraceByChannel (Math|Vector|MakeVector _returnvalue_7 _returnvalue_6 1e+04) (Math|Vector|MakeVector _returnvalue_7 _returnvalue_6 0.0) "TraceTypeQuery1" false 0 "None"))
      (if (>= (Math|Vector|VectorLength (- (Transformation|GetWorldLocation (Variables|Collision|GetCapsuleComponent)) (.Location (Collision|BreakHitResult _outhit)))) 5e+03)
        (if _returnvalue_8
          (bind _outlaunchvelocity (Game|SuggestProjectileVelocityCustomArc (Transformation|GetWorldLocation (Variables|Collision|GetCapsuleComponent)) (.Location (Collision|BreakHitResult _outhit)) 0.0 0.5))
          (CallFunction|JumpEvent _outlaunchvelocity))
        (else
          (goto _label))))))

(event EventOnLanded
  (params (Hit :type Hit%20Result%20Structure%20%28by%20ref%29))
  (bind _returnvalue (Math|Random|RandomFloatinRange 5e+03 7.5e+03))
  (bind _returnvalue_2 (Math|Random|RandomUnitVector))
  (bind _capsulecomponent (Variables|Collision|GetCapsuleComponent))
  (bind _returnvalue_3 (* _returnvalue_2 _returnvalue))
  (bind _returnvalue_4 (Transformation|GetWorldLocation _capsulecomponent))
  (bind _returnvalue_5 (+ _returnvalue_3 _returnvalue_4))
  (bind _returnvalue_6 (Math|Float|Clamp(Float) (.y _returnvalue_5) -5e+03 5e+03))
  (bind _returnvalue_7 (Math|Float|Clamp(Float) (.x _returnvalue_5) -5e+03 5e+03))
  (switch Utilities|FlowControl|Switch|SwitchonLifeformStates (Variables|Default|GetCurrent%20State) :!label _label
    (:NewEnumerator0
      (bind (_outhit _returnvalue_8) (Collision|LineTraceByChannel (Math|Vector|MakeVector _returnvalue_7 _returnvalue_6 1e+04) (Math|Vector|MakeVector _returnvalue_7 _returnvalue_6 0.0) "TraceTypeQuery1" false 0 "None"))
      (if (>= (Math|Vector|VectorLength (- (Transformation|GetWorldLocation (Variables|Collision|GetCapsuleComponent)) (.Location (Collision|BreakHitResult _outhit)))) 5e+03)
        (if _returnvalue_8
          (bind _outlaunchvelocity (Game|SuggestProjectileVelocityCustomArc (Transformation|GetWorldLocation (Variables|Collision|GetCapsuleComponent)) (.Location (Collision|BreakHitResult _outhit)) 0.0 0.5))
          (CallFunction|JumpEvent _outlaunchvelocity))
        (else
          (goto _label))))))

(fn ConstructionScript)

(fn Jumpnoww
  (params (Velocity1 :type Vector)))