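; Net is an actor, with an instigator, that catches players and removes lifeforms it overlaps.
; Overlap handling runs only with authority.
; A Player other than the instigator gets CaughtInNet called and the net destroys itself.
; An overlapped UnspecifiedLifeform is destroyed, while the net remains.
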(event Collision|EventActorBeginOverlap
  (params (OtherActor :type Actor%20Object%20Reference))
  (Networking|SwitchHasAuthority
    (:Authority
      (bind _asthird_person_character (Utilities|Casting|CastToPlayer OtherActor)
        (:then
          (Utilities|IsValid _asthird_person_character
            (:Is%20Valid
              (if (!= OtherActor (Variables|Actor|GetInstigator))
                (Default|CaughtinNet _asthird_person_character)
                (Actor|DestroyActor)))))
        (:CastFailed
          (bind _asunspecified_lifeform (Utilities|Casting|CastToUnspecifiedLifeform OtherActor))
          (Utilities|IsValid _asunspecified_lifeform
            (:Is%20Valid
              (Actor|DestroyActor _asunspecified_lifeform))))))))

(event EventTick
  (params (DeltaSeconds :type Float%20%28single-precision%29)))

(fn ConstructionScript)